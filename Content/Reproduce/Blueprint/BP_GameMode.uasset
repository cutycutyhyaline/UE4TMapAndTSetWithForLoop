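; Game mode that hosts a reproduction test for TArray, TSet and TMap results assigned to local variables with and without a For Loop.
; FullTest and the SimpleTest variants call the container test functions by unrolled calls and by loops, then print contents or lengths for comparison.
; Fixed variants swap in TSetTestFixed and TMapTestFixed, keeping TArrayTest unchanged.
; BeginPlay runs only FullTestFixed; the other test calls are disconnected.
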(event EventBeginPlay
  (CallFunction|FullTestFixed))

(fn ConstructionScript)

(fn FullTest
  (LocalVariables|SetLocalString "=== Case: Without For Loop ===")
  (bind _outarray (Class|Rep02GameModeBase|TArrayTest))
  (LocalVariables|SetLocalTArray _outarray)
  (bind _outarray_2 (Class|Rep02GameModeBase|TArrayTest 1))
  (LocalVariables|SetLocalTArray _outarray_2)
  (bind _outarray_3 (Class|Rep02GameModeBase|TArrayTest 2))
  (LocalVariables|SetLocalTArray _outarray_3)
  (bind _outarray_4 (Class|Rep02GameModeBase|TArrayTest 3))
  (LocalVariables|SetLocalTArray _outarray_4)
  (bind _outset (Class|Rep02GameModeBase|TSetTest))
  (LocalVariables|SetLocalTSet _outset)
  (bind _outset_2 (Class|Rep02GameModeBase|TSetTest 1))
  (LocalVariables|SetLocalTSet _outset_2)
  (bind _outset_3 (Class|Rep02GameModeBase|TSetTest 2))
  (LocalVariables|SetLocalTSet _outset_3)
  (bind _outset_4 (Class|Rep02GameModeBase|TSetTest 3))
  (LocalVariables|SetLocalTSet _outset_4)
  (bind _outmap (Class|Rep02GameModeBase|TMapTest))
  (LocalVariables|SetLocalTMap _outmap)
  (bind _outmap_2 (Class|Rep02GameModeBase|TMapTest 1))
  (LocalVariables|SetLocalTMap _outmap_2)
  (bind _outmap_3 (Class|Rep02GameModeBase|TMapTest 2))
  (LocalVariables|SetLocalTMap _outmap_3)
  (bind _outmap_4 (Class|Rep02GameModeBase|TMapTest 3))
  (LocalVariables|SetLocalTMap _outmap_4)
  (LocalVariables|SetLocalString (Utilities|String|Append (LocalVariables|GetLocalString) " 
 
TArray : "))
  (for (_array_element _array_index) (LocalVariables|GetLocalTArray)
    (LocalVariables|SetLocalString (Utilities|String|Append (LocalVariables|GetLocalString) " 
" (Utilities|String|Append (Utilities|String|Append "index : " (Utilities|String|ToString(Integer) _array_index)) (Utilities|String|Append " / value : " (Utilities|String|ToString(Integer) _array_element))))))
  (LocalVariables|SetLocalString (Utilities|String|Append (LocalVariables|GetLocalString) " 
 
TSet : "))
  (bind _result (Utilities|Set|ToArray (LocalVariables|GetLocalTSet)))
  (for (_array_element_2 _array_index_2) _result
    (LocalVariables|SetLocalString (Utilities|String|Append (LocalVariables|GetLocalString) " 
" (Utilities|String|Append (Utilities|String|Append "index : " (Utilities|String|ToString(Integer) _array_index_2)) (Utilities|String|Append " / value : " (Utilities|String|ToString(Integer) _array_element_2))))))
  (LocalVariables|SetLocalString (Utilities|String|Append (LocalVariables|GetLocalString) " 
 
TMap : "))
  (bind _keys (Utilities|Map|Keys (LocalVariables|GetLocalTMap)))
  (for (_array_element_3 _array_index_3) _keys
    (LocalVariables|SetLocalString (Utilities|String|Append (LocalVariables|GetLocalString) " 
" (Utilities|String|Append (Utilities|String|Append "index : " (Utilities|String|ToString(Integer) _array_index_3)) (Utilities|String|Append " / key : " (Utilities|String|ToString(Integer) _array_element_3)) (Utilities|String|Append " / value : " (Utilities|String|ToString(Integer) (.Value (Utilities|Map|Find (LocalVariables|GetLocalTMap) _array_element_3))))))))
  (LocalVariables|SetLocalString (Utilities|String|Append (LocalVariables|GetLocalString) " 
 
 
 
=== Case : With For Loop  ==="))
  (for _index (range 0 3)
    (bind _outarray_5 (Class|Rep02GameModeBase|TArrayTest _index))
    (LocalVariables|SetLocalTArray _outarray_5))
  (for _index_2 (range 0 3)
    (bind _outset_5 (Class|Rep02GameModeBase|TSetTest _index_2))
    (LocalVariables|SetLocalTSet _outset_5))
  (for _index_3 (range 0 3)
    (bind _outmap_5 (Class|Rep02GameModeBase|TMapTest _index_3))
    (LocalVariables|SetLocalTMap _outmap_5))
  (LocalVariables|SetLocalString (Utilities|String|Append (LocalVariables|GetLocalString) " 
 
TArray : "))
  (for (_array_element_4 _array_index_4) (LocalVariables|GetLocalTArray)
    (LocalVariables|SetLocalString (Utilities|String|Append (LocalVariables|GetLocalString) " 
" (Utilities|String|Append (Utilities|String|Append "index : " (Utilities|String|ToString(Integer) _array_index_4)) (Utilities|String|Append " / value : " (Utilities|String|ToString(Integer) _array_element_4))))))
  (LocalVariables|SetLocalString (Utilities|String|Append (LocalVariables|GetLocalString) " 
 
TSet : "))
  (bind _result_2 (Utilities|Set|ToArray (LocalVariables|GetLocalTSet)))
  (for (_array_element_5 _array_index_5) _result_2
    (LocalVariables|SetLocalString (Utilities|String|Append (LocalVariables|GetLocalString) " 
" (Utilities|String|Append (Utilities|String|Append "index : " (Utilities|String|ToString(Integer) _array_index_5)) (Utilities|String|Append " / value : " (Utilities|String|ToString(Integer) _array_element_5))))))
  (LocalVariables|SetLocalString (Utilities|String|Append (LocalVariables|GetLocalString) " 
 
TMap : "))
  (bind _keys_2 (Utilities|Map|Keys (LocalVariables|GetLocalTMap)))
  (for (_array_element_6 _array_index_6) _keys_2
    (LocalVariables|SetLocalString (Utilities|String|Append (LocalVariables|GetLocalString) " 
" (Utilities|String|Append (Utilities|String|Append "index : " (Utilities|String|ToString(Integer) _array_index_6)) (Utilities|String|Append " / key : " (Utilities|String|ToString(Integer) _array_element_6)) (Utilities|String|Append " / value : " (Utilities|String|ToString(Integer) (.Value (Utilities|Map|Find (LocalVariables|GetLocalTMap) _array_element_6))))))))
  (Development|PrintString (LocalVariables|GetLocalString) true true "(R=0.000000,G=0.660000,B=1.000000,A=1.000000)" 6e+01))

(fn SimpleTest
  (Utilities|FlowControl|Sequence
    (:then_0
      (bind _outset (Class|Rep02GameModeBase|TSetTest))
      (LocalVariables|SetLocalTSet _outset)
      (bind _outset_2 (Class|Rep02GameModeBase|TSetTest 1))
      (LocalVariables|SetLocalTSet _outset_2)
      (Development|PrintString (Utilities|String|Append "Without For Loop : " (Utilities|String|ToString(Integer) (Utilities|Set|Length (LocalVariables|GetLocalTSet)))) true true "(R=0.000000,G=0.660000,B=1.000000,A=1.000000)" 6e+01))
    (:then_1
      (for _index (range 0 1)
        (bind _outset_3 (Class|Rep02GameModeBase|TSetTest _index))
        (LocalVariables|SetLocalTSet _outset_3))
      (Development|PrintString (Utilities|String|Append "With For Loop : " (Utilities|String|ToString(Integer) (Utilities|Set|Length (LocalVariables|GetLocalTSet)))) true true "(R=0.000000,G=0.660000,B=1.000000,A=1.000000)" 6e+01))))

(fn SimpleTestwithTArray
  (Utilities|FlowControl|Sequence
    (:then_0
      (bind _outset (Class|Rep02GameModeBase|TSetTest))
      (LocalVariables|SetLocalTSet _outset)
      (bind _outset_2 (Class|Rep02GameModeBase|TSetTest 1))
      (LocalVariables|SetLocalTSet _outset_2)
      (Development|PrintString (Utilities|String|Append "Without For Loop : " (Utilities|String|ToString(Integer) (Utilities|Set|Length (LocalVariables|GetLocalTSet)))) true true "(R=0.000000,G=0.660000,B=1.000000,A=1.000000)" 6e+01))
    (:then_1
      (for _index (range 0 1)
        (bind _outset_3 (Class|Rep02GameModeBase|TSetTest _index))
        (LocalVariables|SetLocalTSet _outset_3))
      (Development|PrintString (Utilities|String|Append "With For Loop : " (Utilities|String|ToString(Integer) (Utilities|Set|Length (LocalVariables|GetLocalTSet)))) true true "(R=0.000000,G=0.660000,B=1.000000,A=1.000000)" 6e+01)
      (for _index_2 (range 0 1)
        (bind _outarray (Class|Rep02GameModeBase|TArrayTest _index_2))
        (LocalVariables|SetLocalTArray _outarray))
      (Development|PrintString (Utilities|String|Append "But TArray : " (Utilities|String|ToString(Integer) (Utilities|Array|Length (LocalVariables|GetLocalTArray)))) true true "(R=0.000000,G=0.660000,B=1.000000,A=1.000000)" 6e+01))))

(fn SimpleTestFixed
  (Utilities|FlowControl|Sequence
    (:then_0
      (bind _outset (Class|Rep02GameModeBase|TSetTestFixed))
      (LocalVariables|SetLocalTSet _outset)
      (bind _outset_2 (Class|Rep02GameModeBase|TSetTestFixed 1))
      (LocalVariables|SetLocalTSet _outset_2)
      (Development|PrintString (Utilities|String|Append "Without For Loop : " (Utilities|String|ToString(Integer) (Utilities|Set|Length (LocalVariables|GetLocalTSet)))) true true "(R=0.000000,G=0.660000,B=1.000000,A=1.000000)" 6e+01))
    (:then_1
      (for _index (range 0 1)
        (bind _outset_3 (Class|Rep02GameModeBase|TSetTestFixed _index))
        (LocalVariables|SetLocalTSet _outset_3))
      (Development|PrintString (Utilities|String|Append "With For Loop : " (Utilities|String|ToString(Integer) (Utilities|Set|Length (LocalVariables|GetLocalTSet)))) true true "(R=0.000000,G=0.660000,B=1.000000,A=1.000000)" 6e+01))))

(fn FullTestFixed
  (LocalVariables|SetLocalString "=== Case: Without For Loop ===")
  (bind _outarray (Class|Rep02GameModeBase|TArrayTest))
  (LocalVariables|SetLocalTArray _outarray)
  (bind _outarray_2 (Class|Rep02GameModeBase|TArrayTest 1))
  (LocalVariables|SetLocalTArray _outarray_2)
  (bind _outarray_3 (Class|Rep02GameModeBase|TArrayTest 2))
  (LocalVariables|SetLocalTArray _outarray_3)
  (bind _outarray_4 (Class|Rep02GameModeBase|TArrayTest 3))
  (LocalVariables|SetLocalTArray _outarray_4)
  (bind _outset (Class|Rep02GameModeBase|TSetTestFixed))
  (LocalVariables|SetLocalTSet _outset)
  (bind _outset_2 (Class|Rep02GameModeBase|TSetTestFixed 1))
  (LocalVariables|SetLocalTSet _outset_2)
  (bind _outset_3 (Class|Rep02GameModeBase|TSetTestFixed 2))
  (LocalVariables|SetLocalTSet _outset_3)
  (bind _outset_4 (Class|Rep02GameModeBase|TSetTestFixed 3))
  (LocalVariables|SetLocalTSet _outset_4)
  (bind _outmap (Class|Rep02GameModeBase|TMapTestFixed))
  (LocalVariables|SetLocalTMap _outmap)
  (bind _outmap_2 (Class|Rep02GameModeBase|TMapTestFixed 1))
  (LocalVariables|SetLocalTMap _outmap_2)
  (bind _outmap_3 (Class|Rep02GameModeBase|TMapTestFixed 2))
  (LocalVariables|SetLocalTMap _outmap_3)
  (bind _outmap_4 (Class|Rep02GameModeBase|TMapTestFixed 3))
  (LocalVariables|SetLocalTMap _outmap_4)
  (LocalVariables|SetLocalString (Utilities|String|Append (LocalVariables|GetLocalString) " 
 
TArray : "))
  (for (_array_element _array_index) (LocalVariables|GetLocalTArray)
    (LocalVariables|SetLocalString (Utilities|String|Append (LocalVariables|GetLocalString) " 
" (Utilities|String|Append (Utilities|String|Append "index : " (Utilities|String|ToString(Integer) _array_index)) (Utilities|String|Append " / value : " (Utilities|String|ToString(Integer) _array_element))))))
  (LocalVariables|SetLocalString (Utilities|String|Append (LocalVariables|GetLocalString) " 
 
TSet : "))
  (bind _result (Utilities|Set|ToArray (LocalVariables|GetLocalTSet)))
  (for (_array_element_2 _array_index_2) _result
    (LocalVariables|SetLocalString (Utilities|String|Append (LocalVariables|GetLocalString) " 
" (Utilities|String|Append (Utilities|String|Append "index : " (Utilities|String|ToString(Integer) _array_index_2)) (Utilities|String|Append " / value : " (Utilities|String|ToString(Integer) _array_element_2))))))
  (LocalVariables|SetLocalString (Utilities|String|Append (LocalVariables|GetLocalString) " 
 
TMap : "))
  (bind _keys (Utilities|Map|Keys (LocalVariables|GetLocalTMap)))
  (for (_array_element_3 _array_index_3) _keys
    (LocalVariables|SetLocalString (Utilities|String|Append (LocalVariables|GetLocalString) " 
" (Utilities|String|Append (Utilities|String|Append "index : " (Utilities|String|ToString(Integer) _array_index_3)) (Utilities|String|Append " / key : " (Utilities|String|ToString(Integer) _array_element_3)) (Utilities|String|Append " / value : " (Utilities|String|ToString(Integer) (.Value (Utilities|Map|Find (LocalVariables|GetLocalTMap) _array_element_3))))))))
  (LocalVariables|SetLocalString (Utilities|String|Append (LocalVariables|GetLocalString) " 
 
 
 
=== Case : With For Loop  ==="))
  (for _index (range 0 3)
    (bind _outarray_5 (Class|Rep02GameModeBase|TArrayTest _index))
    (LocalVariables|SetLocalTArray _outarray_5))
  (for _index_2 (range 0 3)
    (bind _outset_5 (Class|Rep02GameModeBase|TSetTestFixed _index_2))
    (LocalVariables|SetLocalTSet _outset_5))
  (for _index_3 (range 0 3)
    (bind _outmap_5 (Class|Rep02GameModeBase|TMapTestFixed _index_3))
    (LocalVariables|SetLocalTMap _outmap_5))
  (LocalVariables|SetLocalString (Utilities|String|Append (LocalVariables|GetLocalString) " 
 
TArray : "))
  (for (_array_element_4 _array_index_4) (LocalVariables|GetLocalTArray)
    (LocalVariables|SetLocalString (Utilities|String|Append (LocalVariables|GetLocalString) " 
" (Utilities|String|Append (Utilities|String|Append "index : " (Utilities|String|ToString(Integer) _array_index_4)) (Utilities|String|Append " / value : " (Utilities|String|ToString(Integer) _array_element_4))))))
  (LocalVariables|SetLocalString (Utilities|String|Append (LocalVariables|GetLocalString) " 
 
TSet : "))
  (bind _result_2 (Utilities|Set|ToArray (LocalVariables|GetLocalTSet)))
  (for (_array_element_5 _array_index_5) _result_2
    (LocalVariables|SetLocalString (Utilities|String|Append (LocalVariables|GetLocalString) " 
" (Utilities|String|Append (Utilities|String|Append "index : " (Utilities|String|ToString(Integer) _array_index_5)) (Utilities|String|Append " / value : " (Utilities|String|ToString(Integer) _array_element_5))))))
  (LocalVariables|SetLocalString (Utilities|String|Append (LocalVariables|GetLocalString) " 
 
TMap : "))
  (bind _keys_2 (Utilities|Map|Keys (LocalVariables|GetLocalTMap)))
  (for (_array_element_6 _array_index_6) _keys_2
    (LocalVariables|SetLocalString (Utilities|String|Append (LocalVariables|GetLocalString) " 
" (Utilities|String|Append (Utilities|String|Append "index : " (Utilities|String|ToString(Integer) _array_index_6)) (Utilities|String|Append " / key : " (Utilities|String|ToString(Integer) _array_element_6)) (Utilities|String|Append " / value : " (Utilities|String|ToString(Integer) (.Value (Utilities|Map|Find (LocalVariables|GetLocalTMap) _array_element_6))))))))
  (Development|PrintString (LocalVariables|GetLocalString) true true "(R=0.000000,G=0.660000,B=1.000000,A=1.000000)" 6e+01))